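; BP_IntroStarEnvironment is a backdrop actor for the intro star environment, with an inverted black sphere and a Niagara star effect that share one opacity.
; BeginPlay puts a dynamic M_UnlitBlack instance on the sphere.
; Tick re-applies StarsEnvironmentOpacity to the material and Niagara parameters every frame, which the author flags as a performance cost.
; An editor preview in the construction script is left disconnected for performance.
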(event `self.ReceiveBeginPlay`
  (`self.SetBackgroundMaterial`))

(event `self.ReceiveTick`
  (params (DeltaSeconds :type "Float (single-precision)"))
  (`self.SetStarsEnvironmentOpacity` (`self.starsEnvironmentOpacity`)))

(fn `SetBackgroundMaterial`
  (bind _returnvalue (`KismetMaterialLibrary.CreateDynamicMaterialInstance` "/Game/Environment/IntroStarEnvironment/M_UnlitBlack.M_UnlitBlack"))
  (bind _output_get (set `self.mat` _returnvalue))
  (`PrimitiveComponent.SetMaterial` (`self.SphereInverted`) 0 _output_get))

(fn `SetStarsEnvironmentOpacity`
  (params (opacity :type "Float (double-precision)" :default 1.0))
  (bind _output_get (set `self.starsEnvironmentOpacity` opacity))
  (`MaterialInstanceDynamic.SetScalarParameterValue` (`self.mat`) "Opacity" _output_get)
  (`NiagaraComponent.SetVariableFloat` (`self.NS_Stars`) "OpacityScale" _output_get))

(fn `UserConstructionScript`)